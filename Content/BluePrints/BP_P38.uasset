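; BP_P38 is a player-controlled P-38 aircraft pawn that flies continuously forward and fires rockets.
; Tick feeds forward movement input scaled by IsBoost, which the Boost action raises while held.
; Roll and Pitch axes apply frame-rate-independent local rotation, and Fire spawns a short-lived BP_Rocket at the Arrow component.
; On BeginPlay, it registers the Right and Left components with BPSceneRotator, presumably to spin the propellers.
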(event EventBeginPlay
  (bind __bp_scenerotator (Variables|Default|Get%20BP_SceneRotator))
  (bind _scenecomponents (Variables|/Game/BluePrints/BP_SceneRotator.BP_SceneRotator_C|GetSceneComponents __bp_scenerotator))
  (Utilities|Array|Add _scenecomponents (Variables|Default|GetRight))
  (Utilities|Array|Add _scenecomponents (Variables|Default|GetLeft)))

(event EventTick
  (params (DeltaSeconds :type Float%20%28single-precision%29))
  (Pawn|Input|AddMovementInput (Transformation|GetActorForwardVector) (Variables|Default|GetIsBoost) false))

(event Input|ActionEvents|InputActionFire
  (params (Key :type Key%20Structure :default "None"))
  (:Pressed
    (bind _returnvalue (Game|SpawnActorfromClass "/Game/BluePrints/BP_Rocket.BP_Rocket_C" (Transformation|GetWorldTransform (Variables|Default|GetArrow)) "Undefined" "MultiplyWithRoot" 0 self))
    (Utilities|IsValid _returnvalue
      (:Is%20Valid
        (Actor|SetLifeSpan _returnvalue 3.0)))))

(event Input|ActionEvents|InputActionBoost
  (params (Key :type Key%20Structure :default "None"))
  (:Pressed
    (Variables|Default|SetIsBoost 1.0))
  (:Released
    (Variables|Default|SetIsBoost 0.5)))

(event Input|AxisEvents|InputAxisRoll
  (params (AxisValue :type Float%20%28single-precision%29))
  (Transformation|AddActorLocalRotation (Math|Rotator|MakeRotator (* (Math|Float|Clamp(Float) AxisValue -1.0) (Utilities|Time|GetWorldDeltaSeconds) (Variables|Default|GetRotSpeed)) 0.0 0.0) false false))

(event Input|AxisEvents|InputAxisPitch
  (params (AxisValue :type Float%20%28single-precision%29))
  (Transformation|AddActorLocalRotation (Math|Rotator|MakeRotator 0.0 (* (Math|Float|Clamp(Float) AxisValue -1.0) (Utilities|Time|GetWorldDeltaSeconds) (Variables|Default|GetRotSpeed)) 0.0) false false))

(fn ConstructionScript)